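; MakeDungeon weapon projectile that handles overlaps on its Sphere and Collision components, ignoring its instigator.
; On authority, it line-traces to an overlapped MDCharacterBase with a valid ability system, then adds that character's hit result to the effect context.
; On remote, it simply destroys itself.
; The gameplay effect application and another destroy call are disconnected, so this graph applies no effect.
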(event OnComponentBeginOverlap(Collision)
  (params (OverlappedComponent :type Primitive%20Component%20Object%20Reference) (OtherActor :type Actor%20Object%20Reference) (OtherComp :type Primitive%20Component%20Object%20Reference) (OtherBodyIndex :type Integer) (bFromSweep :type Boolean) (SweepResult :type Hit%20Result%20Structure%20%28by%20ref%29))
  (if (!= OtherActor (Game|GetInstigator))
    (Networking|SwitchHasAuthority
      (:Authority
        (bind _asmdcharacter_base (Utilities|Casting|CastToMDCharacterBase OtherActor))
        (if (Utilities|IsValid (Ability|GetAbilitySystemComponent _asmdcharacter_base))
          (bind _outhits (Class|KismetSystemLibrary|LineTraceMultiforObjects (Transformation|GetActorLocation) (Transformation|GetActorLocation _asmdcharacter_base) (Utilities|Array|MakeArray "ObjectTypeQuery3") false 0 "None" true "(R=1.000000,G=0.000000,B=0.000000,A=1.000000)" "(R=0.000000,G=1.000000,B=0.000000,A=1.000000)" 2.0))
          (bind _array_element (Utilities|Array|ForEachLoopwithBreak _outhits :!label _label)
            (:LoopBody
              (if (== (.HitActor (Collision|BreakHitResult _array_element)) _asmdcharacter_base)
                (Variables|Default|SetFinal%20Hit _array_element)
                (goto _label Break)))
            (:Completed
              (bind _returnvalue (Class|AbilitySystemBlueprintLibrary|GetEffectContext))
              (Class|AbilitySystemBlueprintLibrary|EffectContextAddHitResult _returnvalue (Variables|Default|GetFinal%20Hit) false)))))
      (:Remote
        (Actor|DestroyActor)))))

(event OnComponentBeginOverlap(Sphere)
  (params (OverlappedComponent :type Primitive%20Component%20Object%20Reference) (OtherActor :type Actor%20Object%20Reference) (OtherComp :type Primitive%20Component%20Object%20Reference) (OtherBodyIndex :type Integer) (bFromSweep :type Boolean) (SweepResult :type Hit%20Result%20Structure%20%28by%20ref%29))
  (if (!= (stale OnComponentBeginOverlap(Collision) OtherActor) (Game|GetInstigator))
    (Networking|SwitchHasAuthority
      (:Authority
        (bind _asmdcharacter_base (Utilities|Casting|CastToMDCharacterBase (stale OnComponentBeginOverlap(Collision) OtherActor)))
        (if (Utilities|IsValid (Ability|GetAbilitySystemComponent _asmdcharacter_base))
          (bind _outhits (Class|KismetSystemLibrary|LineTraceMultiforObjects (Transformation|GetActorLocation) (Transformation|GetActorLocation _asmdcharacter_base) (Utilities|Array|MakeArray "ObjectTypeQuery3") false 0 "None" true "(R=1.000000,G=0.000000,B=0.000000,A=1.000000)" "(R=0.000000,G=1.000000,B=0.000000,A=1.000000)" 2.0))
          (bind _array_element (Utilities|Array|ForEachLoopwithBreak _outhits :!label _label)
            (:LoopBody
              (if (== (.HitActor (Collision|BreakHitResult _array_element)) _asmdcharacter_base)
                (Variables|Default|SetFinal%20Hit _array_element)
                (goto _label Break)))
            (:Completed
              (bind _returnvalue (Class|AbilitySystemBlueprintLibrary|GetEffectContext))
              (Class|AbilitySystemBlueprintLibrary|EffectContextAddHitResult _returnvalue (Variables|Default|GetFinal%20Hit) false)))))
      (:Remote
        (Actor|DestroyActor)))))

(fn ConstructionScript)