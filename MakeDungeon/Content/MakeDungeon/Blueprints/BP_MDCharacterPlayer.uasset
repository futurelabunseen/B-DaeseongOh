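; Player character Blueprint for MakeDungeon that sets Motion Warping targets toward the mouse cursor when skill inputs start.
; A helper traces under the cursor, flattens the hit to the actor's height and computes a look-at rotation.
; Skill 02 warps "Move" to the cursor with a two-handed sword tag on the ability system, otherwise "NoMove" turns in place.
; Skill 03 always uses "NoMove", and the attack input is empty.
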(event Input|EnhancedActionEvents|EnhancedInputActionIA_Skill_03
  (params (ActionValue :type Boolean) (ElapsedSeconds :type Float%20%28double-precision%29) (TriggeredSeconds :type Float%20%28double-precision%29) (InputAction :type Input%20Action%20Object%20Reference :default "/Game/MakeDungeon/Input/Actions/IA_Skill_03.IA_Skill_03"))
  (:Started
    (bind (_mwc _actorlocation _cursorlocation _lookatrotation) (CallFunction|GetCursorLocationandLookatforMotionWarping))
    (Class|MotionWarpingComponent|AddorUpdateWarpTargetfromLocationandRotation _mwc "NoMove" _actorlocation _lookatrotation)))

(event Input|EnhancedActionEvents|EnhancedInputActionIA_Skill_02
  (params (ActionValue :type Boolean) (ElapsedSeconds :type Float%20%28double-precision%29) (TriggeredSeconds :type Float%20%28double-precision%29) (InputAction :type Input%20Action%20Object%20Reference :default "/Game/MakeDungeon/Input/Actions/IA_Skill_02.IA_Skill_02"))
  (:Started
    (bind (_mwc _actorlocation _cursorlocation _lookatrotation) (CallFunction|GetCursorLocationandLookatforMotionWarping))
    (if (GameplayTags|HasMatchingGameplayTag (Ability|GetAbilitySystemComponent 0) "(TagName=\"Weapon.Type.TwoHandedSword\")")
      (Class|MotionWarpingComponent|AddorUpdateWarpTargetfromLocationandRotation _mwc "Move" _cursorlocation _lookatrotation)
      (else
        (Class|MotionWarpingComponent|AddorUpdateWarpTargetfromLocationandRotation _mwc "NoMove" _actorlocation _lookatrotation)))))

(event Input|EnhancedActionEvents|EnhancedInputActionIA_Attack
  (params (ActionValue :type Boolean) (ElapsedSeconds :type Float%20%28double-precision%29) (TriggeredSeconds :type Float%20%28double-precision%29) (InputAction :type Input%20Action%20Object%20Reference :default "/Game/MakeDungeon/Input/Actions/IA_Attack.IA_Attack")))

(event EventBeginPlay)

(event Collision|EventActorBeginOverlap
  (params (OtherActor :type Actor%20Object%20Reference)))

(event EventTick
  (params (DeltaSeconds :type Float%20%28single-precision%29)))

(fn ConstructionScript)

(fn GetCursorLocationandLookatforMotionWarping
  (bind _returnvalue (Transformation|GetActorLocation))
  (bind _returnvalue_2 (Game|GetPlayerController 0))
  (bind _z (Math|Vector|BreakVector _returnvalue))
  (bind _hitresult (Game|Player|GetHitResultUnderCursorbyChannel _returnvalue_2 "TraceTypeQuery1" true))
  (bind _location (Collision|BreakHitResult _hitresult))
  (bind (_x _y) (Math|Vector|BreakVector _location))
  (bind _returnvalue_3 (Math|Vector|MakeVector _x _y _z))
  (return (Variables|Default|GetMWC) _returnvalue _returnvalue_3 (Math|Rotator|FindLookatRotation _returnvalue _returnvalue_3)))